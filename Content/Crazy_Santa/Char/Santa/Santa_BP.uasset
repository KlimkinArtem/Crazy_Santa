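; Santa character Blueprint that handles a melee pick attack.
; PickAttackAnim plays a great sword slash montage behind a DoOnce that ResetPickAttack re-arms, while PickAttack_ calls PickAttack, defined outside this graph, with sphere parameters.
; Right mouse fires a debug-drawn line trace from the pick sound socket, with its result unused.
; A disconnected camera-direction trace that spawns a radial force actor at impact never runs.
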(event `PickAttackAnim`
  (`/Engine/EditorBlueprintResources/StandardMacros.DoOnce` false :!label _label
    (:`Completed`
      (`self.PlayAnimMontage` "/Game/Crazy_Santa/Char/Santa/Animations/Action/Great_Sword_Slash_Montage.Great_Sword_Slash_Montage"))))

(event `ResetPickAttack`
  (goto _label :!via `Reset`))

(event `Key|LeftMouseButton`
  (params (Key :type "Key Structure")))

(event `PickAttack_`
  (`self.PickAttack` 25.0 16))

(event `Key|RightMouseButton`
  (params (Key :type "Key Structure"))
  (bind _mesh (`self.Mesh`))
  (bind _returnvalue (`SceneComponent.GetSocketLocation` _mesh "PickSoundSocket"))
  (:`Pressed`
    (`KismetSystemLibrary.LineTraceSingle` :`Start` _returnvalue :`End` (+ _returnvalue (* (* (`KismetMathLibrary.GetForwardVector` (`SceneComponent.GetSocketRotation` _mesh "None")) (1.0 0.0 1.0)) 5000.0)) :`TraceChannel` "TraceTypeQuery1" :`DrawDebugType` "ForDuration")))

(fn `UserConstructionScript`)